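; Light actor Blueprint that cycles its main light through green, orange and red at runtime, like a traffic light.
; The construction script applies the Color variable to that light and uses ToggleVisibility to show or hide both it and a spotlight component.
; BeginPlay then overrides the color in an endless loop, built by wiring one-second Delay nodes back to the first color change.
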(event EventBeginPlay
  (bind _lightcomponent1 (Variables|Default|GetLightComponent1))
  (Rendering|Components|Light|SetLightColor _lightcomponent1 "(R=0.108777,G=0.854993,B=0.017333,A=1.000000)" true :!label _label)
  (Utilities|FlowControl|Delay 1.0)
  (Rendering|Components|Light|SetLightColor _lightcomponent1 "(R=0.822857,G=0.226325,B=0.000000,A=1.000000)" true)
  (Utilities|FlowControl|Delay 1.0)
  (Rendering|Components|Light|SetLightColor _lightcomponent1 "(R=0.811429,G=0.000000,B=0.000000,A=1.000000)" true)
  (Utilities|FlowControl|Delay 1.0)
  (goto _label))

(fn ConstructionScript
  (Rendering|Components|Light|SetLightColor (Variables|Default|GetLightComponent1) (Variables|Default|GetColor) true)
  (Rendering|SetVisibility (Variables|Default|GetSpotLightComponent) (Variables|Default|GetToggle%20Visibility) false))