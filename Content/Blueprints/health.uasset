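; A health pickup Blueprint that restores player health when touched.
; Its static mesh spins by adding a fixed yaw step to its world rotation every Tick, so the spin speed depends on frame rate.
; When the trigger box overlaps a PlayerCharacter, it passes HealthToAdd to IncreasePlayerHealth and then destroys itself.
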(event OnComponentBeginOverlap(TriggerBox_CollisionComp)
  (params (OverlappedComponent :type Primitive%20Component%20Object%20Reference) (OtherActor :type Actor%20Object%20Reference) (OtherComp :type Primitive%20Component%20Object%20Reference) (OtherBodyIndex :type Integer) (bFromSweep :type Boolean) (SweepResult :type Hit%20Result%20Structure%20%28by%20ref%29))
  (bind _asplayer_character (Utilities|Casting|CastToPlayerCharacter OtherActor))
  (Default|IncreasePlayerHealth _asplayer_character (Variables|Default|GethealthToAdd))
  (Actor|DestroyActor))

(event EventTick
  (params (DeltaSeconds :type Float%20%28single-precision%29))
  (bind _sm_merged_triggerbox_blueprint_staticmeshcomponent0 (Variables|Default|GetSM_MERGED_TriggerBox_Blueprint_StaticMeshComponent0))
  (bind _returnvalue (Transformation|GetWorldRotation _sm_merged_triggerbox_blueprint_staticmeshcomponent0))
  (bind (_roll _pitch _yaw) (Math|Rotator|BreakRotator _returnvalue))
  (Transformation|SetWorldRotation _sm_merged_triggerbox_blueprint_staticmeshcomponent0 (Math|Rotator|MakeRotator _roll _pitch (+ _yaw 1.0)) false false))

(fn ConstructionScript)