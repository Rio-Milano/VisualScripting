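; Key pickup actor that gives the first-person player a key when touched.
; Tick spins the Cube mesh around its vertical axis by a fixed step each frame, independent of delta time.
; When the Box overlaps a FirstPersonCharacter and the key is not Hidden, it writes its KeyNUM into the character's CurrentKey, replacing the previous value, and destroys itself.
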(event OnComponentBeginOverlap(Box)
  (params (OverlappedComponent :type Primitive%20Component%20Object%20Reference) (OtherActor :type Actor%20Object%20Reference) (OtherComp :type Primitive%20Component%20Object%20Reference) (OtherBodyIndex :type Integer) (bFromSweep :type Boolean) (SweepResult :type Hit%20Result%20Structure%20%28by%20ref%29))
  (if (not (Variables|Rendering|GetbHidden))
    (bind _asfirst_person_character (Utilities|Casting|CastToFirstPersonCharacter OtherActor))
    (Variables|/Game/Blueprints/Character/FirstPersonCharacter.FirstPersonCharacter_C|SetcurrentKey _asfirst_person_character (Variables|Default|GetkeyNUM))
    (Actor|DestroyActor)))

(event EventTick
  (params (DeltaSeconds :type Float%20%28single-precision%29))
  (bind _cube (Variables|Default|GetCube))
  (bind _returnvalue (Transformation|GetWorldRotation _cube))
  (bind (_roll _pitch _yaw) (Math|Rotator|BreakRotator _returnvalue))
  (Transformation|SetWorldRotation _cube (Math|Rotator|MakeRotator _roll _pitch (+ _yaw 1.0)) false false))

(fn ConstructionScript)