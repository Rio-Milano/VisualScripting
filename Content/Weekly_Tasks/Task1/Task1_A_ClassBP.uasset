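; A light actor Blueprint from a weekly task that blinks on an endless, uneven timer.
; The construction script applies a default color to the main light and sets the initial visibility of both its light components from a toggle variable.
; On BeginPlay, a looping chain of alternating longer and shorter Delays flips only the main light's visibility, with no Tick or Timer.
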(event EventBeginPlay
  (bind _lightcomponent1 (Variables|Default|GetLightComponent1))
  (Utilities|FlowControl|Delay 5.0 :!label _label)
  (Rendering|ToggleVisibility _lightcomponent1 false)
  (Utilities|FlowControl|Delay 3.0)
  (Rendering|ToggleVisibility _lightcomponent1 false)
  (goto _label))

(fn ConstructionScript
  (Rendering|Components|Light|SetLightColor (Variables|Default|GetLightComponent1) (Variables|Default|GetDefault_Color) true)
  (Rendering|SetVisibility (Variables|Default|GetPointLightComponent) (Variables|Default|GetVisibility_toggle) false))