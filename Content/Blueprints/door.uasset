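; Interactable door actor that the player opens and closes, with an optional lock tied to a key number.
; A trigger box enables input and shows an interaction widget while the player character overlaps it.
; Interact plays or reverses a timeline that yaws the mesh and flips the open state when finished, with a creak sound.
; A locked door unlocks permanently when the player's current key matches, otherwise it plays an attempt sound.
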(event OnComponentBeginOverlap(Box1)
  (params (OverlappedComponent :type Primitive%20Component%20Object%20Reference) (OtherActor :type Actor%20Object%20Reference) (OtherComp :type Primitive%20Component%20Object%20Reference) (OtherBodyIndex :type Integer) (bFromSweep :type Boolean) (SweepResult :type Hit%20Result%20Structure%20%28by%20ref%29))
  (bind _returnvalue (Game|GetPlayerController 0))
  (Utilities|Casting|CastToPlayerCharacter OtherActor)
  (Input|EnableInput _returnvalue)
  (bind _returnvalue_2 (UserInterface|CreateWidget "/Game/Blueprints/interactionUI.interactionUI_C" _returnvalue))
  (UserInterface|Viewport|AddtoViewport _returnvalue_2 0))

(event OnComponentEndOverlap(Box1)
  (params (OverlappedComponent :type Primitive%20Component%20Object%20Reference) (OtherActor :type Actor%20Object%20Reference) (OtherComp :type Primitive%20Component%20Object%20Reference) (OtherBodyIndex :type Integer))
  (Utilities|Casting|CastToPlayerCharacter OtherActor)
  (Input|DisableInput (Game|GetPlayerController 0))
  (Widget|RemovefromParent (stale OnComponentBeginOverlap(Box1) _returnvalue_2)))

(event Input|ActionEvents|InputActioninteract
  (params (Key :type Key%20Structure :default "None"))
  (bind _staticmesh (Variables|Default|GetStaticMesh))
  (bind _returnvalue (Transformation|GetWorldLocation _staticmesh))
  ;[1 1 1] Open Door
  (:Pressed
    (if (Variables|Default|GetdoorOpen)
      (Audio|PlaySoundatLocation "/Game/Sounds/Wood_Door_Creak_Open__SOUND_EFFECT_-_AudioTrimmer_com_.Wood_Door_Creak_Open__SOUND_EFFECT_-_AudioTrimmer_com_" _returnvalue "0, 0, 0" 1.0 1.0 0.0 0 0 0)
      (bind _newtrack_0 (Timeline|move%20door Reverse)
        (:Update
          (Transformation|SetRelativeRotation (Variables|Default|GetStaticMesh) (Math|Rotator|MakeRotator 0.0 0.0 _newtrack_0) false false))
        (:Finished
          (if (Variables|Default|GetdoorOpen)
            (Variables|Default|SetdoorOpen false)
            (else
              (Variables|Default|SetdoorOpen true)))))
      (else
        (bind _asplayer_character (Utilities|Casting|CastToPlayerCharacter (Game|GetPlayerCharacter 0)))
        (if (Variables|Default|Getunlocked)
          (Audio|PlaySoundatLocation "/Game/Sounds/Wood_Door_Creak_Open__SOUND_EFFECT_-_AudioTrimmer_com_.Wood_Door_Creak_Open__SOUND_EFFECT_-_AudioTrimmer_com_" _returnvalue "0, 0, 0" 1.0 1.0 0.0 0 0 0 :!label _label)
          (Timeline|move%20door Play)
          (elif (== (Variables|/Game/PlayerCharacter/Blueprints/PlayerCharacter.PlayerCharacter_C|GetcurrentKey _asplayer_character) (Variables|Default|GetkeyNumRequired))
            (Variables|Default|Setunlocked true)
            (goto _label)
            (else
              (Audio|PlaySoundatLocation "/Game/Sounds/doot_open_attem.doot_open_attem" _returnvalue "0, 0, 0" 1.0 1.0 0.0 0 0 0))))))))

(fn ConstructionScript)