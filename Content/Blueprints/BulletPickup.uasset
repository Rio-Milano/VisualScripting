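; Bullet pickup actor that gives ammo to the player who walks into it.
; Overlapping its trigger box casts to PlayerCharacter, awards AmmoToGive through AwardPlayerAmmo and destroys the pickup.
; Two text renders show the amount with a "Bullets" suffix, set in the construction script and again every tick.
; Tick also spins the merged static mesh by adding a fixed yaw step each frame, independent of delta time.
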(event OnComponentBeginOverlap(TriggerBox_CollisionComp)
  (params (OverlappedComponent :type Primitive%20Component%20Object%20Reference) (OtherActor :type Actor%20Object%20Reference) (OtherComp :type Primitive%20Component%20Object%20Reference) (OtherBodyIndex :type Integer) (bFromSweep :type Boolean) (SweepResult :type Hit%20Result%20Structure%20%28by%20ref%29))
  (bind _asplayer_character (Utilities|Casting|CastToPlayerCharacter OtherActor))
  (Default|AwardPlayerAmmo _asplayer_character (Variables|Default|GetammoToGive))
  (Actor|DestroyActor))

(event EventTick
  (params (DeltaSeconds :type Float%20%28single-precision%29))
  (bind _sm_merged_triggerbox_blueprint_staticmeshcomponent0 (Variables|Default|GetSM_MERGED_TriggerBox_Blueprint_StaticMeshComponent0))
  (bind _returnvalue (Transformation|GetWorldRotation _sm_merged_triggerbox_blueprint_staticmeshcomponent0))
  (bind (_roll _pitch _yaw) (Math|Rotator|BreakRotator _returnvalue))
  (Rendering|Components|TextRender|SetText (Variables|Default|GetTextRender1) (Utilities|Text|ToText(String) (Utilities|String|Append (Utilities|String|ToString(Integer) (Variables|Default|GetammoToGive)) " Bullets")))
  (Rendering|Components|TextRender|SetText (Variables|Default|GetTextRender) (Utilities|Text|ToText(String) (Utilities|String|Append (Utilities|String|ToString(Integer) (Variables|Default|GetammoToGive)) " Bullets")))
  (Transformation|SetWorldRotation _sm_merged_triggerbox_blueprint_staticmeshcomponent0 (Math|Rotator|MakeRotator _roll _pitch (+ _yaw 1.0)) false false))

(fn ConstructionScript
  (bind _ammotogive (Variables|Default|GetammoToGive))
  (bind _returnvalue (Utilities|String|ToString(Integer) _ammotogive))
  (bind _returnvalue_2 (Utilities|String|Append _returnvalue " Bullets"))
  (bind _returnvalue_3 (Utilities|Text|ToText(String) _returnvalue_2))
  (Rendering|Components|TextRender|SetText (Variables|Default|GetTextRender1) _returnvalue_3)
  (Rendering|Components|TextRender|SetText (Variables|Default|GetTextRender) _returnvalue_3))