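; Shootable target actor that slides along its local Y axis and counts toward a kill goal that reveals a key.
; A timeline started on BeginPlay drives the slide, reversing when finished and replaying after a delay.
; AnyDamage drains Health; at zero it applies a downward impulse, destroys itself and increments FirstPersonCharacter's Kills, unhiding the Key at ten.
; An older line-trace hit reaction remains disconnected.
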(event Custom|eventMove
  (bind _newtrack_0 (Timeline|Timeline_0 Reverse)
    (:Update
      (Transformation|SetRelativeLocation (Variables|Default|Gettarget) (Math|Vector|MakeVector 0.0 _newtrack_0 0.0) false false))
    (:Finished
      (CallFunction|EventMove)
      (Utilities|FlowControl|Delay 3.0)
      (Timeline|Timeline_0 Play))))

(event EventBeginPlay
  (bind _newtrack_0 (Timeline|Timeline_0 Play)
    (:Update
      (Transformation|SetRelativeLocation (Variables|Default|Gettarget) (Math|Vector|MakeVector 0.0 _newtrack_0 0.0) false false))
    (:Finished
      (CallFunction|EventMove)
      (Utilities|FlowControl|Delay 3.0)
      (Timeline|Timeline_0 Play))))

(event EventTick
  (params (DeltaSeconds :type Float%20%28single-precision%29))
  ;[1 1 1] Line Trace method
)

(event Game|Damage|EventAnyDamage
  (params (Damage :type Float%20%28single-precision%29) (DamageType :type Damage%20Type%20Object%20Reference) (InstigatedBy :type Controller%20Object%20Reference) (DamageCauser :type Actor%20Object%20Reference))
  (bind _target (Variables|Default|Gettarget))
  ;[1 1 1] shoot
  (if (not (Variables|Default|GetisDying))
    (Variables|Default|Sethealth (- (Variables|Default|Gethealth) Damage))
    (if (not (> (Variables|Default|Gethealth) 0.0))
      (Variables|Default|SetisDying true)
      (Physics|SetSimulatePhysics _target true)
      (Physics|AddImpulse _target "0.000000,0.000000,-10000.000000" "None" false)
      (Actor|DestroyActor)
      (bind _asfirst_person_character (Utilities|Casting|CastToFirstPersonCharacter (Game|Player|GetPlayerPawn 0)))
      (Variables|/Game/Blueprints/Character/FirstPersonCharacter.FirstPersonCharacter_C|Setkills _asfirst_person_character (+ (Variables|/Game/Blueprints/Character/FirstPersonCharacter.FirstPersonCharacter_C|Getkills _asfirst_person_character) 1))
      (if (>= (Variables|/Game/Blueprints/Character/FirstPersonCharacter.FirstPersonCharacter_C|Getkills _asfirst_person_character) 10)
        (Rendering|SetActorHiddenInGame (Variables|Default|Getkey) false)))))

(fn ConstructionScript)